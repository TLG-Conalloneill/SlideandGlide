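; BP_WallLampGreen is a wall lamp actor with a configurable spot light, set up at construction rather than during play.
; Its construction script checks TurnOn and either applies the exposed intensity, rotation, outer cone angle and attenuation radius variables to the SpotLight, or sets its intensity to zero.
; The event graph holds only empty default events, so the actor has no runtime logic.
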(event EventBeginPlay)

(event Collision|EventActorBeginOverlap
  (params (OtherActor :type Actor%20Object%20Reference)))

(event EventTick
  (params (DeltaSeconds :type Float%20%28single-precision%29)))

(fn ConstructionScript
  (bind _spotlight (Variables|Default|GetSpotLight))
  (if (Variables|Default|GetTurn%20On?)
    (Rendering|Components|Light|SetIntensity (Variables|Default|GetSpotLight) (Variables|Default|GetNew%20Intensity))
    (Transformation|SetRelativeRotation _spotlight (Variables|Default|GetNew%20Rotation) false false)
    (Rendering|Lighting|SetOuterConeAngle _spotlight (Variables|Default|GetNew%20Outer%20Cone%20Angle))
    (Rendering|Lighting|SetAttenuationRadius (Variables|Default|GetSpotLight) (Variables|Default|GetNew%20Radius))
    (else
      (Rendering|Components|Light|SetIntensity (Variables|Default|GetSpotLight) 0.0))))