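; BP_LevelComplete is a level-end goal: a tumbling cube with a trigger box that completes the level when the player character overlaps it.
; Tick spins the cube with randomized per-axis rotation rates.
; On overlap it pauses the MyGameMode timer, waits briefly, then clears widgets, disables player input, shows a Continue button widget and sets the game mode's Level1Done flag.
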(event OnComponentBeginOverlap(Box)
  (params (OverlappedComponent :type Primitive%20Component%20Object%20Reference) (OtherActor :type Actor%20Object%20Reference) (OtherComp :type Primitive%20Component%20Object%20Reference) (OtherBodyIndex :type Integer) (bFromSweep :type Boolean) (SweepResult :type Hit%20Result%20Structure%20%28by%20ref%29))
  (bind _asbp_third_person_character (Utilities|Casting|CastToBP_ThirdPersonCharacter OtherActor))
  (if (== _asbp_third_person_character OtherActor)
    (bind _asmy_game_mode (Utilities|Casting|CastToMyGameMode (Game|GetGameMode)))
    (Variables|/Game/-OurWork-/Sam/CheckPointSystem/MyGameMode.MyGameMode_C|SetPauseTimer? _asmy_game_mode true)
    (Utilities|FlowControl|Delay 2.5)
    (Viewport|RemoveAllWidgets)
    (Input|DisableInput (Game|GetPlayerCharacter 0) 0)
    (bind _returnvalue (UserInterface|CreateWidget "/Game/-OurWork-/Sam/UI/ContinueButtonWidget.ContinueButtonWidget_C"))
    (UserInterface|Viewport|AddtoViewport _returnvalue 0)
    (bind _asmy_game_mode_2 (Utilities|Casting|CastToMyGameMode (Game|GetGameMode)))
    (Variables|/Game/-OurWork-/Sam/CheckPointSystem/MyGameMode.MyGameMode_C|SetLevel%201%20done _asmy_game_mode_2 true)))

(event EventTick
  (params (DeltaSeconds :type Float%20%28single-precision%29))
  (bind _returnvalue (Math|Random|RandomFloatinRange 1e+02 1.2e+02))
  (bind _returnvalue_2 (* DeltaSeconds _returnvalue))
  (Transformation|AddLocalRotation (Variables|Default|GetCube) (Math|Rotator|MakeRotator _returnvalue_2 (* _returnvalue_2 -1.0) _returnvalue_2) false false))

(fn ConstructionScript)