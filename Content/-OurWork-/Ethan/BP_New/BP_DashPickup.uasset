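; BP_DashPickup is a spinning pickup that grants the player the dash ability.
; Tick applies a randomized yaw rotation each frame, and the construction script colors a Laser effect green and points it upward as a beam.
; When the player character overlaps the Box, it sets HasDash on BP_ThirdPersonCharacter, shows the dash HUD, plays a pickup sound and destroys itself.
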(event OnComponentBeginOverlap(Box)
  (params (OverlappedComponent :type Primitive%20Component%20Object%20Reference) (OtherActor :type Actor%20Object%20Reference) (OtherComp :type Primitive%20Component%20Object%20Reference) (OtherBodyIndex :type Integer) (bFromSweep :type Boolean) (SweepResult :type Hit%20Result%20Structure%20%28by%20ref%29))
  (if (== OtherActor (Game|GetPlayerCharacter 0))
    (bind _asbp_third_person_character (Utilities|Casting|CastToBP_ThirdPersonCharacter OtherActor))
    (Variables|/Game/ThirdPerson/Blueprints/BP_ThirdPersonCharacter.BP_ThirdPersonCharacter_C|SetHasDash? _asbp_third_person_character true)
    (Default|ShowDashHUD (Variables|/Game/ThirdPerson/Blueprints/BP_ThirdPersonCharacter.BP_ThirdPersonCharacter_C|GetHUDVar _asbp_third_person_character))
    (Audio|PlaySound2D "/Engine/VREditor/Sounds/UI/Object_PickUp.Object_PickUp" 1.0 1.0 0.0 0 0)
    (Actor|DestroyActor)))

(event EventTick
  (params (DeltaSeconds :type Float%20%28single-precision%29))
  (Transformation|AddActorLocalRotation (Math|Rotator|MakeRotator 0.0 0.0 (* DeltaSeconds (Math|Random|RandomFloatinRange 1e+02 1.2e+02))) false false))

(fn ConstructionScript
  (Effects|Components|ParticleSystem|SetColorParameter (Variables|Default|Getlaser) "colour" "(R=0.030759,G=0.600694,B=0.000000,A=1.000000)")
  (Effects|Components|ParticleSystem|SetVectorParameter (Variables|Default|Getlaser) "laserEnd" (+ (* (Transformation|GetActorUpVector) 2e+02) (Transformation|GetWorldLocation (Variables|Default|Getlaser)))))