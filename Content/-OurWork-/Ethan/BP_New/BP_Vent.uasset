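; BP_Vent is a vent that launches BP_ThirdPersonCharacter upward when it enters the Box trigger.
; Begin overlap, gated by the character's IsVentJumping flag, overrides velocity with LaunchVelocityZ and scaled-down horizontal velocity, then calls VentJumpStart.
; End overlap clears the flag and, after a delay, calls VentJumpEnd on the character cached by begin overlap.
; Three earlier iterations using DoOnce and AirControl changes remain disconnected.
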(event OnComponentBeginOverlap(Box)
  (params (OverlappedComponent :type Primitive%20Component%20Object%20Reference) (OtherActor :type Actor%20Object%20Reference) (OtherComp :type Primitive%20Component%20Object%20Reference) (OtherBodyIndex :type Integer) (bFromSweep :type Boolean) (SweepResult :type Hit%20Result%20Structure%20%28by%20ref%29))
  ;[0 0.2792 1] Used
  (bind _asbp_third_person_character (Utilities|Casting|CastToBP_ThirdPersonCharacter OtherActor))
  (if (not (Variables|/Game/ThirdPerson/Blueprints/BP_ThirdPersonCharacter.BP_ThirdPersonCharacter_C|GetIsVentJumping? _asbp_third_person_character))
    (Character|LaunchCharacter _asbp_third_person_character (Math|Vector|MakeVector (* (.x (Variables|/Script/Engine.MovementComponent|GetVelocity (Variables|/Script/Engine.Character|GetCharacterMovement _asbp_third_person_character))) 0.3) (* (.y (Variables|/Script/Engine.MovementComponent|GetVelocity (Variables|/Script/Engine.Character|GetCharacterMovement _asbp_third_person_character))) 0.3) (Variables|Default|GetLaunch%20Velocity%20Z)) true true)
    (Default|VentJumpStart _asbp_third_person_character)
    (Variables|/Game/ThirdPerson/Blueprints/BP_ThirdPersonCharacter.BP_ThirdPersonCharacter_C|SetIsVentJumping? _asbp_third_person_character true)))

(event OnComponentEndOverlap(Box)
  (params (OverlappedComponent :type Primitive%20Component%20Object%20Reference) (OtherActor :type Actor%20Object%20Reference) (OtherComp :type Primitive%20Component%20Object%20Reference) (OtherBodyIndex :type Integer))
  ;[0 0.2792 1] Used
  (bind _asbp_third_person_character (Utilities|Casting|CastToBP_ThirdPersonCharacter OtherActor))
  (Variables|/Game/ThirdPerson/Blueprints/BP_ThirdPersonCharacter.BP_ThirdPersonCharacter_C|SetIsVentJumping? _asbp_third_person_character false)
  (Utilities|FlowControl|Delay 2.5)
  (Default|VentJumpEnd (stale OnComponentBeginOverlap(Box) _asbp_third_person_character)))

(fn ConstructionScript)