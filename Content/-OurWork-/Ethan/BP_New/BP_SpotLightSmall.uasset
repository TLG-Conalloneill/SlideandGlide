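; BP_SpotLightSmall is a configurable spotlight whose look is set entirely in the construction script, with no runtime logic.
; It applies exposed-style variables for attenuation radius, intensity and outer cone angle to its SpotLight component.
; A priority chain of color booleans (White, Red, Blue, Yellow, Pink, Purple) picks a preset tint, with the first true one winning.
; The cone angle is applied only when one of those color flags is set.
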(event EventBeginPlay)

(fn ConstructionScript
  (bind _spotlight (Variables|Default|GetSpotLight))
  (Rendering|Lighting|SetAttenuationRadius (Variables|Default|GetSpotLight) (Variables|Default|GetNew%20Radius))
  (Rendering|Components|Light|SetIntensity (Variables|Default|GetSpotLight) (Variables|Default|GetNew%20Intensity))
  (if (Variables|Default|GetWhite)
    (Rendering|Components|Light|SetLightColor _spotlight "(R=1.000000,G=1.000000,B=1.000000,A=1.000000)" true)
    (Rendering|Lighting|SetOuterConeAngle _spotlight (Variables|Default|GetNew%20Outer%20Cone%20Angle) :!label _label)
    (elif (Variables|Default|GetRed)
      (Rendering|Components|Light|SetLightColor (Variables|Default|GetSpotLight) "(R=1.000000,G=0.073000,B=0.088665,A=1.000000)" true)
      (goto _label)
      (elif (Variables|Default|GetBlue)
        (Rendering|Components|Light|SetLightColor (Variables|Default|GetSpotLight) "(R=0.204274,G=0.368666,B=0.687500,A=1.000000)" true)
        (goto _label)
        (elif (Variables|Default|GetYellow)
          (Rendering|Components|Light|SetLightColor (Variables|Default|GetSpotLight) "(R=1.000000,G=0.812798,B=0.307468,A=1.000000)" true)
          (goto _label)
          (elif (Variables|Default|GetPink)
            (Rendering|Components|Light|SetLightColor (Variables|Default|GetSpotLight) "(R=1.000000,G=0.493746,B=0.802849,A=1.000000)" true)
            (goto _label)
            (elif (Variables|Default|GetPurple)
              (Rendering|Components|Light|SetLightColor (Variables|Default|GetSpotLight) "(R=0.436197,G=0.172612,B=1.000000,A=1.000000)" true)
              (goto _label))))))))