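; Light Blueprint that makes its PointLight flicker by repeatedly switching between two intensity levels.
; The Construction Script sets the starting brightness from NewIntensity.
; Tick feeds chained Delays that drop the light to LowIntensity, then briefly after raise it to NewIntensity0, a separate variable from the starting one.
; The flicker repeats without a timer or loop because Tick re-arms each latent Delay once it finishes.
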(event EventTick
  (params (DeltaSeconds :type Float%20%28single-precision%29))
  (Utilities|FlowControl|Delay 0.8)
  (Rendering|Components|Light|SetIntensity (Variables|Default|GetPointLight) (Variables|Default|GetLowIntensity))
  (Utilities|FlowControl|Delay 0.25)
  (Rendering|Components|Light|SetIntensity (Variables|Default|GetPointLight) (Variables|Default|GetNew%20Intensity_0)))

(fn ConstructionScript
  (Rendering|Components|Light|SetIntensity (Variables|Default|GetPointLight) (Variables|Default|GetNew%20Intensity)))