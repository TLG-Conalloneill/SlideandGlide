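; BP_WallRotator is a button that rotates a linked wall when the third-person character steps into its trigger box.
; On overlap it casts the other actor to BP_ThirdPersonCharacter, then switches its mesh to a green material and plays a turn-on sound.
; It then calls RotateWall on the WhichWall reference.
; Nothing here resets the material or blocks repeat triggers, so each new overlap calls the rotation again.
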(event OnComponentBeginOverlap(Box)
  (params (OverlappedComponent :type Primitive%20Component%20Object%20Reference) (OtherActor :type Actor%20Object%20Reference) (OtherComp :type Primitive%20Component%20Object%20Reference) (OtherBodyIndex :type Integer) (bFromSweep :type Boolean) (SweepResult :type Hit%20Result%20Structure%20%28by%20ref%29))
  (bind _asbp_third_person_character (Utilities|Casting|CastToBP_ThirdPersonCharacter OtherActor))
  (if (== _asbp_third_person_character OtherActor)
    (CallFunction|ButtonPress)
    (bind _output_get (Variables|Default|SetWhich%20Wall (Variables|Default|GetWhich%20Wall)))
    (Default|RotateWall _output_get)))

(event Custom|ButtonPress
  (Rendering|Material|SetMaterial (Variables|Default|GetStaticMesh) 0 "/Game/-OurWork-/Ethan/Materials/MI_Green.MI_Green")
  (Audio|PlaySoundatLocation "/Game/-OurWork-/Ethan/Audio_Import/ButtonTurnOn.ButtonTurnOn" "0, 0, 0" "0, 0, 0" 1.0 1.0 0.1 0 0 0 0))

(fn ConstructionScript)