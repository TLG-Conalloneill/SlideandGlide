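; BP_ZipLine is a zip line that carries BP_ThirdPersonCharacter along a spline when it overlaps, if PlayAtBeginning is set.
; The Move_Elevator timeline maps its alpha to spline distance and sets the character root's relative location from local-space spline points.
; Separate events play the timeline or conditionally reverse it.
; The construction script builds hidden-in-game spline mesh segments between points, with mesh assignment left disconnected.
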(event OnComponentBeginOverlap(Spline)
  (params (OverlappedComponent :type Primitive%20Component%20Object%20Reference) (OtherActor :type Actor%20Object%20Reference) (OtherComp :type Primitive%20Component%20Object%20Reference) (OtherBodyIndex :type Integer) (bFromSweep :type Boolean) (SweepResult :type Hit%20Result%20Structure%20%28by%20ref%29))
  (bind _spline (Variables|Default|GetSpline))
  (Utilities|Casting|CastToBP_ThirdPersonCharacter OtherActor)
  (Utilities|FlowControl|Sequence
    (:then_0
      (Components|Timeline|SetPlayRate (Variables|Default|GetMove_Elevator) (/ 1.0 (Variables|Elevator|GetPlayRate%20seconds))))
    (:then_1
      (if (Variables|Spline|GetPlay_At_Beginning)
        (bind _move (Timeline|Move_Elevator Play)
          (:Update
            (bind _asbp_third_person_character (Utilities|Casting|CastToBP_ThirdPersonCharacter OtherActor))
            (Transformation|SetRelativeLocation (Variables|/Script/Engine.Actor|GetRootComponent _asbp_third_person_character) (Spline|GetLocationatDistanceAlongSpline _spline (* _move (Spline|GetSplineLength _spline)) "Local") false false)
            (Rendering|SetVisibility (Variables|/Script/Engine.Actor|GetRootComponent _asbp_third_person_character) true false)))))))

(event Custom|OpenGate
  (bind _spline (Variables|Default|GetSpline))
  (bind _move (Timeline|Move_Elevator Play)
    (:Update
      (bind _asbp_third_person_character (Utilities|Casting|CastToBP_ThirdPersonCharacter (stale OnComponentBeginOverlap(Spline) OtherActor)))
      (Transformation|SetRelativeLocation (Variables|/Script/Engine.Actor|GetRootComponent _asbp_third_person_character) (Spline|GetLocationatDistanceAlongSpline _spline (* _move (Spline|GetSplineLength _spline)) "Local") false false)
      (Rendering|SetVisibility (Variables|/Script/Engine.Actor|GetRootComponent _asbp_third_person_character) true false))))

(event Custom|Play_Animation
  (bind _spline (Variables|Default|GetSpline))
  (bind _move (Timeline|Move_Elevator Play)
    (:Update
      (bind _asbp_third_person_character (Utilities|Casting|CastToBP_ThirdPersonCharacter (stale OnComponentBeginOverlap(Spline) OtherActor)))
      (Transformation|SetRelativeLocation (Variables|/Script/Engine.Actor|GetRootComponent _asbp_third_person_character) (Spline|GetLocationatDistanceAlongSpline _spline (* _move (Spline|GetSplineLength _spline)) "Local") false false)
      (Rendering|SetVisibility (Variables|/Script/Engine.Actor|GetRootComponent _asbp_third_person_character) true false))))

(event Custom|Set_PlayRate
  (Components|Timeline|SetPlayRate (Variables|Default|GetMove_Elevator) (/ 1.0 (Variables|Elevator|GetPlayRate%20seconds))))

(event Custom|CloseGate
  (bind _spline (Variables|Default|GetSpline))
  (if (Variables|Default|GetReverse?)
    (bind _move (Timeline|Move_Elevator Reverse)
      (:Update
        (bind _asbp_third_person_character (Utilities|Casting|CastToBP_ThirdPersonCharacter (stale OnComponentBeginOverlap(Spline) OtherActor)))
        (Transformation|SetRelativeLocation (Variables|/Script/Engine.Actor|GetRootComponent _asbp_third_person_character) (Spline|GetLocationatDistanceAlongSpline _spline (* _move (Spline|GetSplineLength _spline)) "Local") false false)
        (Rendering|SetVisibility (Variables|/Script/Engine.Actor|GetRootComponent _asbp_third_person_character) true false)))))

(event EventBeginPlay)

(fn ConstructionScript
  (bind _spline (Variables|Default|GetSpline))
  (for _index (range 0 (- (Spline|GetNumberOfSplinePoints (Variables|Default|GetSpline)) 2))
    (bind _returnvalue (AddComponent|AddSplineMeshComponent false))
    (SplineMesh|SetForwardAxis _returnvalue (Variables|Spline|GetAxis) true)
    (Transformation|AttachComponentToComponent _returnvalue (Variables|Default|GetSpline) "None" "KeepRelative" "KeepRelative" "KeepRelative" true)
    (SplineMesh|SetStartandEnd _returnvalue (Spline|GetLocationatSplinePoint _spline _index "Local") (Spline|GetTangentatSplinePoint _spline _index "Local") (Spline|GetLocationatSplinePoint _spline (+ _index 1) "Local") (Spline|GetTangentatSplinePoint _spline (+ _index 1) "Local") true :!class /Script/Engine.SplineMeshComponent)
    (Development|SetHiddeninGame _returnvalue true false)))