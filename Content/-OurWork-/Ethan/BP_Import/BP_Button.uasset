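; BP_Button is a button that opens the level's gate when the third-person character overlaps its box.
; The press turns the mesh green and plays a turn-on sound, then calls OpenGate on BP_Gate and ChangeColour on BP_ControlPanel, each found with GetActorOfClass.
; A check of the character's Interacting flag is left disconnected, so overlap alone triggers the button.
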(event OnComponentBeginOverlap(Box)
  (params (OverlappedComponent :type Primitive%20Component%20Object%20Reference) (OtherActor :type Actor%20Object%20Reference) (OtherComp :type Primitive%20Component%20Object%20Reference) (OtherBodyIndex :type Integer) (bFromSweep :type Boolean) (SweepResult :type Hit%20Result%20Structure%20%28by%20ref%29))
  (bind _asbp_third_person_character (Utilities|Casting|CastToBP_ThirdPersonCharacter OtherActor))
  (CallFunction|ButtonPress)
  (bind _returnvalue (Actor|GetActorOfClass "/Game/-OurWork-/Ethan/BP_Import/BP_Gate.BP_Gate_C"))
  (Default|OpenGate _returnvalue)
  (bind _returnvalue_2 (Actor|GetActorOfClass "/Game/-OurWork-/Ethan/BP_Import/BP_ControlPanel.BP_ControlPanel_C"))
  (Default|ChangeColour _returnvalue_2))

(event Custom|ButtonPress
  (Rendering|Material|SetMaterial (Variables|Default|GetStaticMesh) 0 "/Game/-OurWork-/Ethan/Materials/MI_Green.MI_Green")
  (Audio|PlaySoundatLocation "/Game/-OurWork-/Ethan/Audio_Import/ButtonTurnOn.ButtonTurnOn" "0, 0, 0" "0, 0, 0" 1.0 1.0 0.1 0 0 0 0))

(fn ConstructionScript)