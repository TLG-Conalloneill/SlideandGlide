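; Zipline actor that tells actors overlapping its Box to start riding between its two top attach points.
; InitCable pins the Zipline cable between those points at construction and BeginPlay.
; Box overlap sends SetZiplineMessage with endpoints ordered by a ForwardInput check, whose facing-versus-input dot product is left unwired; leaving sends a default message.
; Debug prints remain, and cable overlap only prints.
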(event OnComponentBeginOverlap(Zipline)
  (params (OverlappedComponent :type Primitive%20Component%20Object%20Reference) (OtherActor :type Actor%20Object%20Reference) (OtherComp :type Primitive%20Component%20Object%20Reference) (OtherBodyIndex :type Integer) (bFromSweep :type Boolean) (SweepResult :type Hit%20Result%20Structure%20%28by%20ref%29))
  (Utilities|Casting|CastToBP_ThirdPersonCharacter OtherActor)
  (Development|PrintString "Hello"))

(event OnComponentBeginOverlap(Box)
  (params (OverlappedComponent :type Primitive%20Component%20Object%20Reference) (OtherActor :type Actor%20Object%20Reference) (OtherComp :type Primitive%20Component%20Object%20Reference) (OtherBodyIndex :type Integer) (bFromSweep :type Boolean) (SweepResult :type Hit%20Result%20Structure%20%28by%20ref%29))
  (bind _attachstarttop (Variables|Default|GetAttachStartTop))
  (bind _attachendtop (Variables|Default|GetAttachEndTop))
  (bind _returnvalue (Transformation|GetWorldLocation _attachstarttop))
  (bind _returnvalue_2 (Transformation|GetWorldLocation _attachendtop))
  ;[1 1 1] Start
  (Development|PrintString "Hello")
  (if (> (Utilities|ForwardInput) 0.0)
    (Class|BPIZiplineRider|SetZipline(Message) OtherActor true _returnvalue _returnvalue_2 true)
    (Development|PrintString "set 0" true true "(R=1.000000,G=0.000000,B=0.182927,A=1.000000)")
    (else
      (Class|BPIZiplineRider|SetZipline(Message) OtherActor true _returnvalue_2 _returnvalue false)
      (Development|PrintString "set 1" true true "(R=1.000000,G=0.009549,B=0.000000,A=1.000000)"))))

(event OnComponentEndOverlap(Box)
  (params (OverlappedComponent :type Primitive%20Component%20Object%20Reference) (OtherActor :type Actor%20Object%20Reference) (OtherComp :type Primitive%20Component%20Object%20Reference) (OtherBodyIndex :type Integer))
  ;[1 1 1] Start
  (Class|BPIZiplineRider|SetZipline(Message) OtherActor false "0, 0, 0" "0, 0, 0" false)
  (Development|PrintString "nothoing"))

(event EventBeginPlay
  (Utilities|InitCable))

(fn ConstructionScript
  (Utilities|InitCable)
  (Variables|Default|SetTransform (Transformation|GetWorldTransform (Variables|Default|GetBox))))