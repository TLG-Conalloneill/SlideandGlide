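; Gate actor that slides a static mesh along an editable spline to open, and back to close when Reverse is enabled.
; A timeline, scaled to last PlayRateSeconds, drives the mesh's distance along the spline and can optionally play on BeginPlay.
; The construction script adds a spline mesh component per segment to trace the path, hidden in game.
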(event Custom|OpenGate
  (bind _staticmesh (Variables|Default|GetStaticMesh))
  (bind _spline (Variables|Default|GetSpline))
  (bind _move (Timeline|Move_Elevator Play)
    (:Update
      (Transformation|SetRelativeLocation _staticmesh (Spline|GetLocationatDistanceAlongSpline _spline (* _move (Spline|GetSplineLength _spline)) "Local") false false)
      (Rendering|SetVisibility _staticmesh true false))))

(event Custom|Play_Animation
  (bind _staticmesh (Variables|Default|GetStaticMesh))
  (bind _spline (Variables|Default|GetSpline))
  (bind _move (Timeline|Move_Elevator Play)
    (:Update
      (Transformation|SetRelativeLocation _staticmesh (Spline|GetLocationatDistanceAlongSpline _spline (* _move (Spline|GetSplineLength _spline)) "Local") false false)
      (Rendering|SetVisibility _staticmesh true false))))

(event Custom|Set_PlayRate
  (Components|Timeline|SetPlayRate (Variables|Default|GetMove_Elevator) (/ 1.0 (Variables|Elevator|GetPlayRate%20seconds))))

(event Custom|CloseGate
  (bind _staticmesh (Variables|Default|GetStaticMesh))
  (bind _spline (Variables|Default|GetSpline))
  (if (Variables|Default|GetReverse?)
    (bind _move (Timeline|Move_Elevator Reverse)
      (:Update
        (Transformation|SetRelativeLocation _staticmesh (Spline|GetLocationatDistanceAlongSpline _spline (* _move (Spline|GetSplineLength _spline)) "Local") false false)
        (Rendering|SetVisibility _staticmesh true false)))))

(event EventBeginPlay
  (bind _staticmesh (Variables|Default|GetStaticMesh))
  (bind _spline (Variables|Default|GetSpline))
  (Utilities|FlowControl|Sequence
    (:then_0
      (Components|Timeline|SetPlayRate (Variables|Default|GetMove_Elevator) (/ 1.0 (Variables|Elevator|GetPlayRate%20seconds))))
    (:then_1
      (if (Variables|Spline|GetPlay_At_Beginning)
        (bind _move (Timeline|Move_Elevator Play)
          (:Update
            (Transformation|SetRelativeLocation _staticmesh (Spline|GetLocationatDistanceAlongSpline _spline (* _move (Spline|GetSplineLength _spline)) "Local") false false)
            (Rendering|SetVisibility _staticmesh true false)))))))

(fn ConstructionScript
  (bind _spline (Variables|Default|GetSpline))
  (for _index (range 0 (- (Spline|GetNumberOfSplinePoints (Variables|Default|GetSpline)) 2))
    (bind _returnvalue (AddComponent|AddSplineMeshComponent false))
    (Components|StaticMesh|SetStaticMesh _returnvalue 0)
    (SplineMesh|SetForwardAxis _returnvalue (Variables|Spline|GetAxis) true)
    (Transformation|AttachComponentToComponent _returnvalue (Variables|Default|GetSpline) "None" "KeepRelative" "KeepRelative" "KeepRelative" true)
    (SplineMesh|SetStartandEnd _returnvalue (Spline|GetLocationatSplinePoint _spline _index "Local") (Spline|GetTangentatSplinePoint _spline _index "Local") (Spline|GetLocationatSplinePoint _spline (+ _index 1) "Local") (Spline|GetTangentatSplinePoint _spline (+ _index 1) "Local") true :!class /Script/Engine.SplineMeshComponent)
    (Development|SetHiddeninGame _returnvalue true false)))