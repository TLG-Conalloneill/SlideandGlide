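; RespawnPointBP is a checkpoint trigger that updates the respawn location when the third-person character enters its box.
; On overlap it traces 500 units down from SpawnLocArrow and uses the hit location, raised 200 units, as the spawn point.
; It writes that point, with the character's rotation and scale, to MyGameMode's SpawnLocation and prints a debug message.
; The trace result is used without checking for a hit.
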(event OnComponentBeginOverlap(Box)
  (params (OverlappedComponent :type Primitive%20Component%20Object%20Reference) (OtherActor :type Actor%20Object%20Reference) (OtherComp :type Primitive%20Component%20Object%20Reference) (OtherBodyIndex :type Integer) (bFromSweep :type Boolean) (SweepResult :type Hit%20Result%20Structure%20%28by%20ref%29))
  (bind _spawnlocarrow (Variables|Default|GetSpawnLocArrow))
  (bind _returnvalue (Transformation|GetWorldTransform _spawnlocarrow))
  (bind (_x _y _z) (Math|Vector|BreakVector (.location _returnvalue)))
  (bind _asbp_third_person_character (Utilities|Casting|CastToBP_ThirdPersonCharacter OtherActor))
  (bind _asmy_game_mode (Utilities|Casting|CastToMyGameMode (Game|GetGameMode)))
  (bind _outhit (Collision|LineTraceByChannel (.location _returnvalue) (Math|Vector|MakeVector _x _y (- _z 5e+02)) "TraceTypeQuery1" false 0 "None"))
  (Variables|/Game/-OurWork-/Sam/CheckPointSystem/MyGameMode.MyGameMode_C|SetSpawnLocation _asmy_game_mode (Math|Transform|MakeTransform (Math|Vector|MakeVector (.X (Math|Vector|BreakVector (.location _outhit))) (.Y (Math|Vector|BreakVector (.location _outhit))) (+ (.Z (Math|Vector|BreakVector (.location _outhit))) 2e+02)) (.Rotation (Math|Transform|BreakTransform (Transformation|GetActorTransform _asbp_third_person_character))) (.Scale (Math|Transform|BreakTransform (Transformation|GetActorTransform _asbp_third_person_character)))))
  (Development|PrintString "CHECKPOINT" true true "(R=1.000000,G=0.936634,B=0.000000,A=1.000000)"))

(fn ConstructionScript)