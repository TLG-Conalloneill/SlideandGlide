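; Navigation guide actor that marks the navmesh route from the player character to itself with particle waypoints.
; BuildNav finds the path synchronously, turns its points into a spline and spawns a few evenly spaced particle components along it.
; After a short Delay, it clears the spline and destroys those waypoints.
; BeginPlay binds BuildNav to a looping timer whose time is zero.
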(event Custom|BuildNav
  (bind _path_points (CallFunction|FindPathFunction))
  (CallFunction|BuildSpline _path_points)
  (CallFunction|BuildPath)
  (Utilities|FlowControl|Delay 1.0)
  (CallFunction|ClearSpline))

(event EventBeginPlay
  (Utilities|Time|SetTimerbyEvent (delegate Custom|BuildNav) 0.0 true))

(fn ConstructionScript)

(fn FindPathFunction
  (bind _returnvalue (Class|NavigationSystemV1|FindPathtoActorSynchronously (Transformation|GetActorLocation (Game|GetPlayerCharacter 0)) self 5e+01 0 0))
  (return (Variables|/Script/NavigationSystem.NavigationPath|GetPathPoints _returnvalue)))

(fn BuildSpline
  (params (PathPoints :type Array%20of%20Vectors))
  (for _array_element PathPoints
    (Spline|AddSplinePoint (Variables|Default|GetSpline) _array_element "World" true)))

(fn BuildPath
  (for _index (range 0 2)
    (bind _returnvalue (AddComponent|AddParticleSystemComponent false))
    (Transformation|SetWorldLocation _returnvalue (Spline|GetLocationatDistanceAlongSpline (Variables|Default|GetSpline) (* (+ _index 1) 3e+02) "World") false false)
    (Utilities|Array|Add (Variables|Default|GetWayPointList) _returnvalue)))

(fn ClearSpline
  (bind _waypointlist (Variables|Default|GetWayPointList))
  (Spline|ClearSplinePoints (Variables|Default|GetSpline) true)
  (for _array_element _waypointlist
    (Components|DestroyComponent _array_element))
  (Utilities|Array|Clear _waypointlist))