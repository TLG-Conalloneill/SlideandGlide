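; Parent weapon Blueprint that, when fired, throws a BP_DaggerThrow toward the screen center and adds hit effects.
; CenterOfScreen line-traces from the player camera to find the aim point, which orients WeaponArrow and the spawned dagger.
; A sphere trace along the arrow, ignoring the player, picks impact effects by Enemy or Target tag.
; Its Damage and WeaponInteract interface checks lead nowhere, and the TakeDamage call is unconnected, so it deals no damage itself.
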(event Custom|weapon%20goes%20pew
  (bind _weaponarrow (Variables|Default|GetWeaponArrow))
  (bind _returnvalue (Math|Vector|GetForwardVector _weaponarrow))
  (bind _returnvalue_2 (Transformation|GetWorldLocation _weaponarrow))
  (bind _returnvalue_3 (* _returnvalue 2e+06))
  (Development|PrintString "shoot")
  (bind _returnvalue_4 (CallFunction|CenterOfScreen))
  (Transformation|SetWorldRotation (Variables|Default|GetWeaponArrow) (Math|Rotator|FindLookatRotation _returnvalue_2 _returnvalue_4) false false)
  (Game|SpawnActorfromClass "/Game/-OurWork-/Ethan/BP_New/BP_DaggerThrow.BP_DaggerThrow_C" (Math|Transform|MakeTransform (Transformation|GetWorldLocation (Variables|Default|GetWeaponArrow)) (Math|Rotator|FindLookatRotation _returnvalue_2 _returnvalue_4) "1.000000,1.000000,1.000000") "AlwaysSpawn" 0 0)
  (bind _outhit (Collision|SphereTraceByChannel _returnvalue_2 (+ _returnvalue_2 _returnvalue_3) 5.0 "TraceTypeQuery1" false (Variables|Default|GetActors%20to%20Ignore) "None"))
  (if (.bblockinghit _outhit)
    (Utilities|IsValid (.hitactor _outhit)
      (:Is%20Valid
        (if (Actor|ActorHasTag (.hitactor _outhit) "Enemy")
          (Niagara|SpawnSystematLocation 0 (.location _outhit))
          (if (Utilities|DoesObjectImplementInterface (.hitactor _outhit) "/Game/-OurWork-/Ethan/BP_Import/Interfaces/Damage.Damage_C") :!label _label
            _)
          (elif (Actor|ActorHasTag (.hitactor _outhit) "Target")
            (Niagara|SpawnSystematLocation 0 (.location _outhit))
            (if (Utilities|DoesObjectImplementInterface (.hitactor _outhit) "/Game/-OurWork-/Sam/Interface/Weapon-Interact.Weapon-Interact_C")
              _)
            (else
              (Effects|SpawnEmitteratLocation 0 (Math|Vector|SelectVector (.location _outhit) _returnvalue_3 (.bblockinghit _outhit)))
              (goto _label))))))))

(event EventBeginPlay
  (Utilities|Array|Add (Variables|Default|GetActors%20to%20Ignore) (Game|GetPlayerCharacter 0))
  (Development|PrintString "Ignore Self"))

(fn ConstructionScript)

(fn CenterOfScreen
  (bind _returnvalue (Game|GetPlayerController 0))
  (bind _playercameramanager (Variables|/Script/Engine.PlayerController|GetPlayerCameraManager _returnvalue))
  (bind _rootcomponent (Variables|/Script/Engine.Actor|GetRootComponent _playercameramanager))
  (bind _rootcomponent_2 (Variables|/Script/Engine.Actor|GetRootComponent _playercameramanager))
  (bind _returnvalue_2 (Transformation|GetWorldLocation _rootcomponent))
  (bind _returnvalue_3 (Math|Vector|GetForwardVector _rootcomponent_2))
  (bind _returnvalue_4 (* _returnvalue_3 5e+05))
  (bind _returnvalue_5 (+ _returnvalue_2 _returnvalue_4))
  (bind _outhit (Collision|LineTraceByChannel (+ _returnvalue_2 (* _returnvalue_3 1e+02)) _returnvalue_5 "TraceTypeQuery1" false (Variables|Default|GetActors%20to%20Ignore) "None"))
  (return (Math|Vector|SelectVector (.location _outhit) _returnvalue_5 (.bblockinghit _outhit))))